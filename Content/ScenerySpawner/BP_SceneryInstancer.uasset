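; BP_SceneryInstancer is a scenery actor that builds a straight row of a randomly sized number of instanced meshes ("poles").
; OnDespawn picks a count between MinPoles and MaxPoles, then adds instances end to end along local X, spaced by mesh bounds, without clearing earlier ones.
; It caches the row's size in ImmediateBounds, returned by GetFullBounds.
; OnRespawn is empty, and PrintDebug prints the actor's bounds size.
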(event EventBeginPlay
  (|CallParentFunction) ; This node is disabled and will not be called.\nDrag off pins to build functionality.
)

(event Collision|EventActorBeginOverlap
  (params (OtherActor :type Actor%20Object%20Reference))
  (|CallParentFunction OtherActor) ; This node is disabled and will not be called.\nDrag off pins to build functionality.
)

(event EventTick
  (params (DeltaSeconds :type Float%20%28single-precision%29))
  (|CallParentFunction DeltaSeconds) ; This node is disabled and will not be called.\nDrag off pins to build functionality.
)

(event EventOnRespawn)

(event EventOnDespawn
  (bind _instancedstaticmesh (Variables|Default|GetInstancedStaticMesh))
  (bind _staticmesh (Variables|/Script/Engine.StaticMeshComponent|GetStaticMesh _instancedstaticmesh))
  (bind _returnvalue (StaticMesh|GetBounds _staticmesh))
  (bind _boxextent (Math|BoxSphereBounds|BreakBoxSphereBounds _returnvalue))
  (bind (_x _y _z) (Math|Vector|BreakVector _boxextent))
  (bind _output_get (Variables|Default|SetCurrentPoles (Math|Random|RandomIntegerinRange (Variables|Default|GetMinPoles) (Variables|Default|GetMaxPoles))))
  (for _index (range 0 _output_get)
    (bind _output_get_2 (Variables|Default|SetMeshExtents _boxextent))
    (Components|InstancedStaticMesh|AddInstance (Variables|Default|GetInstancedStaticMesh) (Math|Transform|MakeTransform (* (* _output_get_2 (Math|Conversions|ToFloat(Integer) _index) 2.0) (Class|KismetMathLibrary|VectorForward))) false))
  (Variables|Default|SetImmediateBounds (* (Math|Vector|MakeVector (* (Variables|Default|GetCurrentPoles) _x) _y _z) 2.0)))

(fn ConstructionScript
  (|CallParentFunction))

(fn PrintDebug
  (Development|PrintString (Utilities|String|ToString(Vector) (* (.BoxExtent (Collision|GetActorBounds false false)) 2.0))))

(fn GetFullBounds
  (return (Variables|Default|GetImmediateBounds)))