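; BP_Bird is a bird actor that flies along a spline path and plays a window-impact sound near the end.
; After a start delay, a timer starts a timeline whose play rate is scaled by the flight duration.
; Timeline alpha drives world position and rotation along the referenced FlyPath spline.
; Once alpha passes 0.8, a DoOnce fires the FMOD impact event at the bird mesh's location.
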(event Custom|FlyAndCrash
  (bind _flypathref (Variables|Default|GetFlyPathRef))
  (bind _flypath (Variables|/Game/Blueprints/BP_BirdPath.BP_BirdPath_C|GetFlyPath _flypathref))
  (Components|Timeline|SetPlayRate (Variables|Default|GetTimeline) (/ 1.0 (Variables|Default|GetDuration)))
  (bind _alpha (Timeline|Timeline PlayFromStart)
    (:Update
      (bind _output_get (Variables|Default|SetAlpha _alpha))
      (Utilities|FlowControl|Sequence
        (:then_0
          (if (> _output_get 0.8)
            (Utilities|FlowControl|DoOnce false
              (:Completed
                (Class|FMODBlueprintStatics|PlayEventatLocation "/Game/FMOD/Events/Mood/sx_mood_impact_bird_window.sx_mood_impact_bird_window" (Math|Conversions|ToTransform(Vector) (Transformation|GetWorldLocation (Variables|Default|GetSM_Bird))))))))
        (:then_1
          (Transformation|SetActorLocationAndRotation (Spline|GetLocationatDistanceAlongSpline _flypath (Math|Float|Lerp 0.0 (Spline|GetSplineLength (Variables|/Game/Blueprints/BP_BirdPath.BP_BirdPath_C|GetFlyPath (Variables|Default|GetFlyPathRef))) (Variables|Default|GetAlpha)) "World") (Spline|GetRotationatDistanceAlongSpline _flypath (Math|Float|Lerp 0.0 (Spline|GetSplineLength (Variables|/Game/Blueprints/BP_BirdPath.BP_BirdPath_C|GetFlyPath (Variables|Default|GetFlyPathRef))) (Variables|Default|GetAlpha)) "World")))))))

(event EventBeginPlay
  (Utilities|Time|SetTimerbyEvent (delegate Custom|FlyAndCrash) (Variables|Default|GetStartDelay)))

(event Collision|EventActorBeginOverlap
  (params (OtherActor :type Actor%20Object%20Reference)))

(event EventTick
  (params (DeltaSeconds :type Float%20%28single-precision%29)))

(fn ConstructionScript)